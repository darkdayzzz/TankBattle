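; Player-controlled tank Blueprint with an orbiting aim camera and a fire action.
; On BeginPlay it passes its Barrel and Turret components to the tank through setter functions.
; Aim axes rotate the camera rig, yaw on the azimuth gimbal and pitch on the spring arm, scaled by delta time.
; The Fire input calls Fire, whose logic lives outside these graphs.
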(event `self.ReceiveBeginPlay`
  (`self.SetBarrelReference` (`self.Barrel`))
  (`self.SetTurretReference` (`self.Turret`)))

(event `InputAxis|AimAzimuth`
  (params (AxisValue :type "Float (single-precision)"))
  ;[1 1 1] Camera movement
  (`SceneComponent.K2_AddLocalRotation` (`self.AzimuthGimbal`) (`KismetMathLibrary.MakeRotator` 0.0 0.0 (* AxisValue (`GameplayStatics.GetWorldDeltaSeconds`) 100.0)) false false))

(event `InputAxis|AimElevation`
  (params (AxisValue :type "Float (single-precision)"))
  ;[1 1 1] Camera movement
  (`SceneComponent.K2_AddLocalRotation` (`self.SpringArm`) (`KismetMathLibrary.MakeRotator` 0.0 (* AxisValue (`GameplayStatics.GetWorldDeltaSeconds`) 75.0)) false false))

(event `InputAction|Fire`
  (params (Key :type "Key Structure" :default "AnyKey"))
  ;[1 1 1] In-game actions
  (:`Pressed`
    (`self.Fire`)))

(fn `UserConstructionScript`)